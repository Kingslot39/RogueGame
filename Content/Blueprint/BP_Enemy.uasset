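; Enemy Blueprint that chases and melee-attacks the player once pawn sensing detects a pawn.
; Each sighting starts an AI move to the player character; the seeing flag is never cleared here.
; On arrival, a sphere trace at the weapon socket damages a third-person character hit as the attack montage starts.
; A CanAttack flag blocks further attacks until a delay of the montage's returned length ends.
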(event `self.PawnSensing.OnSeePawn`
  (params (Pawn :type "Pawn Object Reference"))
  (set `self.isSeeingPlayer` true)
  (`self.FollowPlayer`))

(event `FollowPlayer`
  (if (`self.isSeeingPlayer`)
    (`|AIMoveTo` self (0.0 0.0 0.0) (`GameplayStatics.GetPlayerCharacter` 0) 150.0
      (:`OnSuccess`
        (if (`self.CanAttack`)
          (set `self.CanAttack` false)
          (`self.HitDirection`)
          (bind _returnvalue (`self.PlayAnimMontage` "/Game/Animation/NEWANIMS/EnemyAtk_Montage.EnemyAtk_Montage" 2.0))
          (`KismetSystemLibrary.Delay` _returnvalue)
          (set `self.CanAttack` true))))))

(fn `HitDirection`
  (bind _returnvalue (`SceneComponent.GetSocketLocation` (`self.Mesh`) "Weapon_Socket"))
  (bind _outhit (`KismetSystemLibrary.SphereTraceSingleForObjects` _returnvalue _returnvalue 40.0 (`|MakeArray` "ObjectTypeQuery3" :!type "EObjectTypeQuery Enum")))
  (bind _asbp_third_person_character (cast `/Game/ThirdPerson/Blueprints/BP_ThirdPersonCharacter` (`.HitActor` (`GameplayStatics.BreakHitResult` _outhit))))
  (`GameplayStatics.ApplyDamage` _asbp_third_person_character 5.0 null self))

(fn `UserConstructionScript`)