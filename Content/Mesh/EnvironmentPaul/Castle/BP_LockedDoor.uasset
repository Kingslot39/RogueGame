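; BP_LockedDoor is a castle gate that opens once the player has collected enough keys.
; CollectKey increments a key counter, and the player overlapping the Trigger runs a check of that counter against MaxKeysCollected.
; When the requirement is met, a DoOnce fires OpenDoor, where a timeline lerps the Gate's relative Z location to raise it.
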(event `OpenDoor`
  (bind (_direction _door_increase) (`Timeline|Open Door Anim`)
    (:`Update`
      (`SceneComponent.K2_SetRelativeLocation` (`self.Gate`) (`KismetMathLibrary.MakeVector` 0.0 0.0 (`KismetMathLibrary.Lerp` 0.0 250.0 _door_increase)) false false))))

(event `CollectKey`
  (`/Engine/EditorBlueprintResources/StandardMacros.IncrementInt` (`self.currentKeysCollected`)))

(event `Open Door Check`
  (if (>= (`self.currentKeysCollected`) (`self.maxKeysCollected`))
    (`/Engine/EditorBlueprintResources/StandardMacros.DoOnce` false
      (:`Completed`
        (`self.OpenDoor`)))))

(event `self.Trigger.OnComponentBeginOverlap`
  (params (OverlappedComponent :type "PrimitiveComponent Object Reference") (OtherActor :type "Actor Object Reference") (OtherComp :type "PrimitiveComponent Object Reference") (OtherBodyIndex :type Integer) (bFromSweep :type Boolean) (SweepResult :type "HitResult Structure (by ref)"))
  (if (== OtherActor (`GameplayStatics.GetPlayerCharacter` 0))
    (`self.Open Door Check`)))

(fn `UserConstructionScript`)